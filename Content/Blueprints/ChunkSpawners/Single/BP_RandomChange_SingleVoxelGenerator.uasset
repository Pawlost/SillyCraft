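; Single-chunk voxel spawner Blueprint that keeps randomly editing voxels in its chunk at runtime.
; On BeginPlay it starts a looping timer whose interval is set by ChangeSpeed.
; Each tick of the timer calls ChangeVoxelInChunk on SingleChunkGridPosition with a random position inside a 32-voxel cube and a random name from ChangeVoxelNames.
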(event Custom|CustomEvent
  (bind _change_voxel_names (Variables|Default|GetChange%20Voxel%20Names))
  (Class|ChunkSpawnerBase|ChangeVoxelinChunk (Variables|Default|GetSingleChunkGridPosition) (Utilities|Struct|MakeIntVector (Math|Random|RandomIntegerinRange 0 31) (Math|Random|RandomIntegerinRange 0 31) (Math|Random|RandomIntegerinRange 0 31)) (Utilities|Array|Get(acopy) _change_voxel_names (Math|Random|RandomIntegerinRange 0 (- (Utilities|Array|Length _change_voxel_names) 1)))))

(event EventBeginPlay
  (Utilities|Time|SetTimerbyEvent (delegate Custom|CustomEvent) (Variables|Default|GetChangeSpeed) true))

(fn ConstructionScript)