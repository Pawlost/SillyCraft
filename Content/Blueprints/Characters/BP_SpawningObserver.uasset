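; BP_SpawningObserver is a character that creates a ChunkSpawner and drives where it spawns chunks as the character moves.
; On BeginPlay it spawns the ChunkSpawner at its own transform, then teleports vertically to the highest elevation at that location plus a SpawnAboveGround offset.
; Each Tick, while movement acceleration is nonzero, it passes its current location to the spawner's MoveSpawnToPosition.
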(event EventBeginPlay
  (bind _returnvalue (Transformation|GetActorLocation))
  (bind _returnvalue_2 (Game|SpawnActorfromClass (Variables|Default|GetChunk%20spawner) (Transformation|GetActorTransform) "Undefined" "MultiplyWithRoot" 0 0))
  (bind _output_get (Variables|Default|SetChunkSpawner _returnvalue_2))
  (Transformation|SetActorLocation (Math|Vector|MakeVector (.x _returnvalue) (.y _returnvalue) (+ (Class|ChunkSpawnerBase|GetHighestElevationatLocation _output_get (Transformation|GetActorLocation)) (Variables|Default|GetSpawnAboveGround))) false true))

(event Collision|EventActorBeginOverlap
  (params (OtherActor :type Actor%20Object%20Reference)))

(event EventTick
  (params (DeltaSeconds :type Float%20%28single-precision%29))
  (|CallParentFunction 0.0)
  (if (not (Utilities|Operators|EqualEqual :A (Pawn|Components|CharacterMovement|GetCurrentAcceleration (Variables|Character|GetCharacterMovement))))
    (Class|ChunkSpawnerBase|MoveSpawntoPosition (Variables|Default|GetChunkSpawner) (Transformation|GetActorLocation))))

(fn ConstructionScript
  (|CallParentFunction))