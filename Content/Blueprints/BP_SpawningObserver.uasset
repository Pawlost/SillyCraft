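; BP_SpawningObserver is a movable observer that drives chunk spawning around its own position.
; On BeginPlay it spawns a ChunkSpawner at its transform and stores the reference.
; Each Tick, while its CharacterMovement has non-zero acceleration, it passes its integer-truncated location to the spawner's MoveSpawnToPosition, so updates depend on movement input rather than velocity.
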(event EventBeginPlay
  (bind _returnvalue (Game|SpawnActorfromClass (Variables|Default|GetChunk%20spawner) (Transformation|GetActorTransform) "Undefined" "MultiplyWithRoot" 0 0))
  (Variables|Default|SetChunkSpawner _returnvalue))

(event Collision|EventActorBeginOverlap
  (params (OtherActor :type Actor%20Object%20Reference)))

(event EventTick
  (params (DeltaSeconds :type Float%20%28single-precision%29))
  (if (not (Utilities|Operators|EqualEqual :A (Pawn|Components|CharacterMovement|GetCurrentAcceleration (Variables|Character|GetCharacterMovement))))
    (Class|ChunkSpawnerBase|MoveSpawntoPosition (Variables|Default|GetChunkSpawner) (Class|KismetMathLibrary|FTruncVector (.location (Transformation|GetActorTransform))))))

(fn ConstructionScript
  (|CallParentFunction))